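; Player pawn for a click-to-move action game with melee attacks, health and HUD updates.
; While left mouse is held, a gated Tick walks or runs by distance to the cursor point, or approaches a clicked Enemy, attacking once it overlaps Range.
; Shift-click attacks toward the cursor through a second gate; Attack plays a montage and damages any valid Target.
; Incoming damage lowers health and refreshes the HUD; Q applies self-damage.
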(event OnComponentBeginOverlap(Range)
  (params (OverlappedComponent :type Primitive%20Component%20Object%20Reference) (OtherActor :type Actor%20Object%20Reference) (OtherComp :type Primitive%20Component%20Object%20Reference) (OtherBodyIndex :type Integer) (bFromSweep :type Boolean) (SweepResult :type Hit%20Result%20Structure%20%28by%20ref%29))
  (bind _target (Variables|Default|GetTarget))
  (Utilities|IsValid _target
    (:Is%20Valid
      (if (and (== OtherActor _target) (Actor|ActorHasTag _target "Enemy"))
        (AI|Navigation|StopMovement (Game|GetPlayerController 0))
        (CallFunction|Attack)))))

(event Custom|Attack
  (bind _target (Variables|Default|GetTarget))
  (bind _capsulecomponent (Variables|Collision|GetCapsuleComponent))
  ;[1 1 1] Attack
  (if (not (Variables|Default|GetisAttacking))
    (Variables|Default|SetisAttacking true)
    (Transformation|SetWorldRotation _capsulecomponent (Math|Rotator|MakeRotator 0.0 0.0 (.yaw (Math|Rotator|FindLookatRotation (Transformation|GetWorldLocation _capsulecomponent) (Variables|Default|GetTargetLocation)))) false false)
    (bind _returnvalue (Animation|PlayAnimMontage "/Game/_Main/Player/Animations/Montage_Attack.Montage_Attack" 3.0 "None"))
    (Utilities|IsValid _target
      (:Is%20Valid
        (Game|Damage|ApplyDamage _target (Math|Conversions|ToFloat(Integer) (.damage (Variables|Default|GetStats))) (Game|GetPlayerController 0) self))
      (:Is%20Not%20Valid
        _))
    (Utilities|FlowControl|Delay _returnvalue)
    (Variables|Default|SetisAttacking false)))

(event EventTick
  (params (DeltaSeconds :type Float%20%28single-precision%29))
  (bind _hitresult_hitactor (Utilities|GetClickedActor))
  (Utilities|FlowControl|Gate true
    (:Exit
      (if (not (Game|Player|IsInputKeyDown (Game|GetPlayerController 0) (stale Input|KeyboardEvents|LeftShift Key)))
        (Variables|Default|SetTargetLocation (Utilities|GetDestinationtoMove))
        (Utilities|IsValid _hitresult_hitactor
          (:Is%20Valid
            (Variables|Default|SetTarget _hitresult_hitactor)
            (if (Actor|ActorHasTag _hitresult_hitactor "Enemy")
              (Utilities|MoveandAttack)
              (else
                (Utilities|MovetoClickedPlace :!label _label))))
          (:Is%20Not%20Valid
            (goto _label)))))))

(event Game|Damage|EventAnyDamage
  (params (Damage :type Float%20%28single-precision%29) (DamageType :type Damage%20Type%20Object%20Reference) (InstigatedBy :type Controller%20Object%20Reference) (DamageCauser :type Actor%20Object%20Reference))
  ;[1 0.08854 0.08854] Damage Event
  (Variables|Default|SetCurHealth (- (Variables|Default|GetCurHealth) (Math|Float|Truncate Damage)))
  (Class|BPIHeroInterface|UpdateHud(Message) (Pawn|GetController) (CallFunction|GetHPPercent) (CallFunction|GetResourcePercent)))

(event Input|MouseEvents|LeftMouseButton
  (params (Key :type Key%20Structure :default "None"))
  (bind _hitresult_hitactor (Utilities|GetClickedActor))
  (:Pressed
    (Utilities|FlowControl|Sequence
      (:then_0
        (Variables|Default|SetTarget 0))
      (:then_1
        (Utilities|FlowControl|Gate true) ; enters at Open
      )))
  (:Released
    (Utilities|FlowControl|Gate true) ; enters at Close
  ))

(event Input|KeyboardEvents|Q
  (params (Key :type Key%20Structure :default "None"))
  (bind _self self)
  ;[1 1 1] Selfharm
  (:Pressed
    (Game|Damage|ApplyDamage _self 1e+01 0 _self)))

(event Input|KeyboardEvents|1
  (params (Key :type Key%20Structure :default "None")))

(event Input|KeyboardEvents|2
  (params (Key :type Key%20Structure :default "None")))

(event Input|KeyboardEvents|3
  (params (Key :type Key%20Structure :default "None")))

(event Input|KeyboardEvents|4
  (params (Key :type Key%20Structure :default "None")))

(event Input|KeyboardEvents|LeftShift
  (params (Key :type Key%20Structure :default "None"))
  (bind _returnvalue (Game|GetPlayerController 0))
  (bind _array (Utilities|Array|MakeArray "ObjectTypeQuery3"))
  (bind _hitresult (Class|PlayerController|GetHitResultUnderCursorforObjects _returnvalue _array true))
  ;[1 1 1] Attack on place
  (:Pressed
    (Utilities|FlowControl|Gate true) ; enters at Open
  )
  (:Released
    (Utilities|FlowControl|Gate true) ; enters at Close
  ))

(event Input|MouseEvents|LeftMouseButton
  (params (Key :type Key%20Structure :default "None"))
  (bind _returnvalue (Game|GetPlayerController 0))
  (bind _array (Utilities|Array|MakeArray "ObjectTypeQuery3"))
  (bind _hitresult (Class|PlayerController|GetHitResultUnderCursorforObjects _returnvalue _array true))
  ;[1 1 1] Attack on place
  (:Pressed
    (Utilities|FlowControl|Gate true
      (:Exit
        (Variables|Default|SetTargetLocation (.location (.HitResult (Game|Player|GetHitResultUnderCursorbyChannel _returnvalue "TraceTypeQuery1" true))))
        (Utilities|IsValid (.hitactor _hitresult)
          (:Is%20Valid
            (Variables|Default|SetTarget (.hitactor _hitresult)))
          (:Is%20Not%20Valid
            (AI|Navigation|StopMovement _returnvalue)
            (CallFunction|Attack)))))))

(event Input|KeyboardEvents|LeftShift
  (params (Key :type Key%20Structure :default "None"))
  (bind _hitresult_hitactor (Utilities|GetClickedActor))
  (:Pressed
    (Utilities|FlowControl|Gate true) ; enters at Close
  ))

(fn ConstructionScript)

(fn OnRepCurHealth)

(fn GetHPPercent
  (return (/ (Math|Conversions|ToFloat(Integer) (Variables|Default|GetCurHealth)) (Math|Conversions|ToFloat(Integer) (Variables|Default|GetMaxHealth)))))

(fn GetResourcePercent
  (return (/ (Math|Conversions|ToFloat(Integer) (Variables|Default|GetCurResource)) (Math|Conversions|ToFloat(Integer) (Variables|Default|GetMaxResource)))))